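; BP_EnemyBase is a base enemy that damages the runner character on contact with its DamageCollision component.
; An overlap calls TryHitPlayer, which requires the enemy to be active and casts the other actor to BP_RunnerCharacter before calling ReceiveDamage with DamageAmount.
; An optional HitOnce flag limits damage to a single hit until ResetEnemy reactivates the enemy and clears the consumed hit.
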(event `self.DamageCollision.OnComponentBeginOverlap`
  (params (OverlappedComponent :type "PrimitiveComponent Object Reference") (OtherActor :type "Actor Object Reference") (OtherComp :type "PrimitiveComponent Object Reference") (OtherBodyIndex :type Integer) (bFromSweep :type Boolean) (SweepResult :type "HitResult Structure (by ref)"))
  (`self.TryHitPlayer` OtherActor))

(fn `ResetEnemy`
  (set `self.bIsActive` true)
  (set `self.bHitConsumed` false))

(fn `TryHitPlayer`
  (params (OtherActor :type "Actor Object Reference"))
  (if (and (`self.bIsActive`) (or (not (`self.bHitOnce`)) (not (`self.bHitConsumed`))))
    (bind _asbp_runner_character (cast `/Game/ThirdPerson/Blueprints/BP_RunnerCharacter` OtherActor))
    (set `self.bHitConsumed` true)
    (`/Game/ThirdPerson/Blueprints/BP_RunnerCharacter.ReceiveDamage` _asbp_runner_character (`self.DamageAmount`))))

(fn `UserConstructionScript`)