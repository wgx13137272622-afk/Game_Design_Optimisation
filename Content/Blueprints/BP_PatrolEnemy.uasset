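; Patrol enemy Blueprint that moves along the Y axis, driven by a timeline started on BeginPlay.
; Each update scales PatrolDistance by the timeline alpha and sets the root's relative location from the saved start position.
; The offset vector reuses the start X and Z, so adding it to StartLocation doubles both.
; An overridden ResetEnemy calls the parent, returns to the start and restarts the timeline.
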(event `self.ReceiveBeginPlay`
  (bind (_startlocation_x _startlocation_y _startlocation_z) (`KismetMathLibrary.BreakVector` (`self.StartLocation`)))
  (set `self.StartLocation` (`SceneComponent.RelativeLocation` (`self.DefaultSceneRoot`)))
  (bind (_direction _movementalpha) (`Timeline|TL_PatrolMove` :!via `PlayFromStart`)
    (:`Update`
      (`SceneComponent.K2_SetRelativeLocation` (`self.DefaultSceneRoot`) (+ (`self.StartLocation`) (`KismetMathLibrary.MakeVector` _startlocation_x (* (`self.PatrolDistance`) _movementalpha) _startlocation_z)) false false))))

(fn `ResetEnemy`
  (`parent.ResetEnemy`)
  (`TimelineComponent.Stop` (`self.TL_PatrolMove`))
  (`SceneComponent.K2_SetRelativeLocation` (`self.DefaultSceneRoot`) (`self.StartLocation`) false false)
  (`TimelineComponent.PlayFromStart` (`self.TL_PatrolMove`)))

(fn `UserConstructionScript`
  (`parent.UserConstructionScript`))