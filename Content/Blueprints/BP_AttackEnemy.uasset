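; BP_AttackEnemy is an enemy that makes a one-shot telegraphed attack on the runner character.
; When the runner enters DetectionCollision while IsActive, it latches AttackTriggered, prints debug warnings and waits through a short windup.
; It then briefly enables DamageCollision and damages overlapping runners via a single GetOverlappingActors check rather than continuous hit detection.
; AttackTriggered is never reset here, so the attack does not repeat.
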(event `self.ReceiveBeginPlay`
  (`parent.ReceiveBeginPlay`)
  (`PrimitiveComponent.SetCollisionEnabled` (`self.DamageCollision`) "NoCollision"))

(event `self.DetectionCollision.OnComponentBeginOverlap`
  (params (OverlappedComponent :type "PrimitiveComponent Object Reference") (OtherActor :type "Actor Object Reference") (OtherComp :type "PrimitiveComponent Object Reference") (OtherBodyIndex :type Integer) (bFromSweep :type Boolean) (SweepResult :type "HitResult Structure (by ref)"))
  (cast `/Game/ThirdPerson/Blueprints/BP_RunnerCharacter` OtherActor)
  (if (and (`self.bIsActive`) (not (`self.bAttackTriggered`)))
    (set `self.bAttackTriggered` true)
    (`KismetSystemLibrary.PrintString` "Enemy Detected")
    (`KismetSystemLibrary.PrintString` "Attack Warning!")
    (`KismetSystemLibrary.Delay` 0.6)
    (`PrimitiveComponent.SetCollisionEnabled` (`self.DamageCollision`) "QueryOnly")
    (for _array_element (`PrimitiveComponent.GetOverlappingActors` (`self.DamageCollision`) "/Game/ThirdPerson/Blueprints/BP_RunnerCharacter.BP_RunnerCharacter_C")
      (bind _asbp_runner_character (cast `/Game/ThirdPerson/Blueprints/BP_RunnerCharacter` _array_element))
      (`/Game/ThirdPerson/Blueprints/BP_RunnerCharacter.ReceiveDamage` _asbp_runner_character 1))
    (`KismetSystemLibrary.PrintString` "Attack Active")
    (`KismetSystemLibrary.Delay` 0.3)
    (`PrimitiveComponent.SetCollisionEnabled` (`self.DamageCollision`) "NoCollision")
    (`KismetSystemLibrary.PrintString` "Attack Finished")))

(fn `UserConstructionScript`
  (`parent.UserConstructionScript`))