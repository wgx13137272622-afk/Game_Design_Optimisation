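; BP_Collectible is a pickup that the runner character collects on overlap, with an empty CollectionEffect hook that appears intended for child Blueprints to override.
; An overlap on PickupCollision by a BP_RunnerCharacter calls OnCollected, which uses an IsCollected guard to run the effect once, then hides the actor and disables collision.
; ResetCollectible clears the flag, shows the actor and restores query-only collision, allowing reuse without respawning.
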(event `self.PickupCollision.OnComponentBeginOverlap`
  (params (OverlappedComponent :type "PrimitiveComponent Object Reference") (OtherActor :type "Actor Object Reference") (OtherComp :type "PrimitiveComponent Object Reference") (OtherBodyIndex :type Integer) (bFromSweep :type Boolean) (SweepResult :type "HitResult Structure (by ref)"))
  (bind _asbp_runner_character (cast `/Game/ThirdPerson/Blueprints/BP_RunnerCharacter` OtherActor))
  (`self.OnCollected` _asbp_runner_character))

(fn `CollectionEffect`
  (params (Collector :type "/Game/ThirdPerson/Blueprints/BP_RunnerCharacter Object Reference")))

(fn `OnCollected`
  (params (Collector :type "/Game/ThirdPerson/Blueprints/BP_RunnerCharacter Object Reference"))
  (if (not (`self.bIsCollected`))
    (set `self.bIsCollected` true)
    (`self.CollectionEffect` Collector)
    (`self.SetActorHiddenInGame` true)
    (`PrimitiveComponent.SetCollisionEnabled` (`self.PickupCollision`) "NoCollision")))

(fn `ResetCollectible`
  (set `self.bIsCollected` false)
  (`self.SetActorHiddenInGame` false)
  (`PrimitiveComponent.SetCollisionEnabled` (`self.PickupCollision`) "QueryOnly"))

(fn `UserConstructionScript`)