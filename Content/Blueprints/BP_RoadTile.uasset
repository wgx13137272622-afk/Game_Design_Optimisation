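; BP_RoadTile is a recyclable road segment for a runner game that leapfrogs forward along X once the player has passed it.
; When BP_RunnerCharacter stops overlapping RoadTrigger far enough ahead of the tile's origin, the tile teleports forward by a fixed offset instead of being respawned.
; It then resets its directly attached BP_Collectible and BP_EnemyBase actors so its contents can be reused.
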(event `self.RoadTrigger.OnComponentEndOverlap`
  (params (OverlappedComponent :type "PrimitiveComponent Object Reference") (OtherActor :type "Actor Object Reference") (OtherComp :type "PrimitiveComponent Object Reference") (OtherBodyIndex :type Integer))
  (bind _returnvalue_x (`KismetMathLibrary.BreakVector` (`self.K2_GetActorLocation`)))
  (bind _asbp_runner_character (cast `/Game/ThirdPerson/Blueprints/BP_RunnerCharacter` OtherActor))
  (bind _returnvalue_x_2 (`KismetMathLibrary.BreakVector` (`self.K2_GetActorLocation` _asbp_runner_character)))
  (if (> _returnvalue_x_2 (+ _returnvalue_x 1000.0))
    (`self.K2_SetActorLocation` (+ (`self.K2_GetActorLocation`) (`KismetMathLibrary.MakeVector` 6000.0)))
    (for _array_element (`self.GetAttachedActors` true)
      (bind _asbp_collectible (cast `/Game/Blueprints/BP_Collectible` _array_element)
        (:`then`
          (`/Game/Blueprints/BP_Collectible.ResetCollectible` _asbp_collectible))
        (:`CastFailed`
          (bind _asbp_enemy_base (cast `/Game/Blueprints/BP_EnemyBase` _array_element))
          (`/Game/Blueprints/BP_EnemyBase.ResetEnemy` _asbp_enemy_base))))))

(fn `UserConstructionScript`)